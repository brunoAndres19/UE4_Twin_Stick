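; Projectile Blueprint that can be destroyed by a Shoot event or by overlapping other actors.
; On overlap it destroys itself unless the valid other actor is tagged Player, Enemy or EnemyProjectile.
; The Shoot event destroys it immediately, with no further checks.
; The graph contains no movement or damage logic, and BeginPlay, Tick and the construction script are empty.
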(event EventBeginPlay)

(event Collision|EventActorBeginOverlap
  (params (OtherActor :type Actor%20Object%20Reference))
  (if (Utilities|IsValid OtherActor)
    (if (not (Actor|ActorHasTag OtherActor "Player"))
      (if (not (or (Actor|ActorHasTag OtherActor "Enemy") (Actor|ActorHasTag OtherActor "EnemyProjectile")))
        (Actor|DestroyActor)))))

(event EventTick
  (params (DeltaSeconds :type Float%20%28single-precision%29)))

(event EventShoot
  (Actor|DestroyActor))

(fn ConstructionScript)