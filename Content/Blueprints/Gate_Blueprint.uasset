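; Gate actor that opens when its switch is shot by enough projectiles, optionally after linked enemies are destroyed.
; Destruction events from linked enemies count down to enable the switch, whose material shows its state.
; Tagged projectile overlaps count down to disable the switch and play a timeline that moves the gate along Z from its initial height.
; A separate box overlap only prints a debug greeting.
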(event OnComponentBeginOverlap(Switch)
  (params (OverlappedComponent :type Primitive%20Component%20Object%20Reference) (OtherActor :type Actor%20Object%20Reference) (OtherComp :type Primitive%20Component%20Object%20Reference) (OtherBodyIndex :type Integer) (bFromSweep :type Boolean) (SweepResult :type Hit%20Result%20Structure%20%28by%20ref%29))
  (Utilities|IsValid OtherActor
    (:Is%20Valid
      (if (Variables|Default|GetIsSwitchEnabled)
        (if (Actor|ActorHasTag OtherActor "Projectile")
          (bind _result (Math|Integer|DecrementInt (Variables|Default|GetShootsToOpenGate))
            (:%20%20
              (if (== _result 0)
                (Variables|Default|SetIsSwitchEnabled false)
                (Rendering|Material|SetMaterial (Variables|Default|GetSwitch) 1 "/Game/Materials/DisabledSwitchMaterial.DisabledSwitchMaterial")
                (bind _gatemovement (Timeline|Timeline Play)
                  (:Update
                    (Transformation|SetRelativeLocation (Variables|Default|GetGate) (Math|Vector|MakeVector 0.0 0.0 (- (.Z (Math|Vector|BreakVector (Variables|Default|GetInitialGateLocation))) _gatemovement)) false false)))))))))))

(event OnComponentBeginOverlap(Box)
  (params (OverlappedComponent :type Primitive%20Component%20Object%20Reference) (OtherActor :type Actor%20Object%20Reference) (OtherComp :type Primitive%20Component%20Object%20Reference) (OtherBodyIndex :type Integer) (bFromSweep :type Boolean) (SweepResult :type Hit%20Result%20Structure%20%28by%20ref%29))
  (Development|PrintString "Hello"))

(event Custom|OnLinkedEnemyDestroyed
  (params (DestroyedActor :type Actor%20Object%20Reference))
  (bind _result (Math|Integer|DecrementInt (Variables|Default|GetLinkedEnemiesCount))
    (:%20%20
      (if (== _result 0)
        (Variables|Default|SetIsSwitchEnabled true)
        (Rendering|Material|SetMaterial (Variables|Default|GetSwitch) 1 "/Game/Materials/EnabledSwitchMaterial.EnabledSwitchMaterial")))))

(event EventBeginPlay
  (Variables|Default|SetInitialGateLocation (Transformation|GetWorldLocation (Variables|Default|GetGate)))
  (if (Variables|Default|GetIsSwitchEnabled)
    (Rendering|Material|SetMaterial (Variables|Default|GetSwitch) 1 "/Game/Materials/EnabledSwitchMaterial.EnabledSwitchMaterial")
    (else
      (Rendering|Material|SetMaterial (Variables|Default|GetSwitch) 1 "/Game/Materials/DisabledSwitchMaterial.DisabledSwitchMaterial")))
  (Variables|Default|SetLinkedEnemiesCount (Utilities|Array|Length (Variables|Default|GetLinkedEnemies)))
  (for _array_element (Variables|Default|GetLinkedEnemies)
    (Game|BindEventtoOnDestroyed _array_element (delegate Custom|OnLinkedEnemyDestroyed))))

(event Collision|EventActorBeginOverlap
  (params (OtherActor :type Actor%20Object%20Reference)))

(event EventTick
  (params (DeltaSeconds :type Float%20%28single-precision%29)))

(fn ConstructionScript)