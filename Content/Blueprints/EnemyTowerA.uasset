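; EnemyTowerA is an enemy tower that fires through four child-actor projectile spawners and can be destroyed.
; ActivateEnemy marks it active and activates the spawners in sequence, where a failed cast skips only that spawner.
; While active, each Shoot event decrements ShootsToDestroy, and a Shoot received at zero destroys the actor.
; Shoot does nothing before activation.
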(event EventBeginPlay)

(event Collision|EventActorBeginOverlap
  (params (OtherActor :type Actor%20Object%20Reference)))

(event EventTick
  (params (DeltaSeconds :type Float%20%28single-precision%29)))

(event EventShoot
  (bind _shootstodestroy (Variables|Default|GetShootsToDestroy))
  (if (Variables|Default|GetIsActive)
    (if (== 0 _shootstodestroy)
      (Actor|DestroyActor)
      (else
        (Math|Integer|DecrementInt _shootstodestroy)))))

(event EventActivateEnemy
  (Variables|Default|SetIsActive true)
  (Utilities|FlowControl|Sequence
    (:then_0
      (bind _asprojectile_spawner (Utilities|Casting|CastToProjectileSpawner (Variables|/Script/Engine.ChildActorComponent|GetChildActor (Variables|Default|GetFrontProjectileSpawner))))
      (Default|Activate _asprojectile_spawner))
    (:then_1
      (bind _asprojectile_spawner_2 (Utilities|Casting|CastToProjectileSpawner (Variables|/Script/Engine.ChildActorComponent|GetChildActor (Variables|Default|GetFrontProjectileSpawner1))))
      (Default|Activate _asprojectile_spawner_2))
    (:then_2
      (bind _asprojectile_spawner_3 (Utilities|Casting|CastToProjectileSpawner (Variables|/Script/Engine.ChildActorComponent|GetChildActor (Variables|Default|GetFrontProjectileSpawner2))))
      (Default|Activate _asprojectile_spawner_3))
    (:then_3
      (bind _asprojectile_spawner_4 (Utilities|Casting|CastToProjectileSpawner (Variables|/Script/Engine.ChildActorComponent|GetChildActor (Variables|Default|GetFrontProjectileSpawner3))))
      (Default|Activate _asprojectile_spawner_4))))

(fn ConstructionScript)