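; ProjectileSpawner is an actor that repeatedly spawns a configurable projectile class at a fixed interval once activated.
; Activate sets the IsActive flag, after which Tick accumulates delta time and spawns when it reaches SpawnTime, then resets the timer.
; Each projectile takes the spawner's rotation and appears at its location plus SpawnOffset, which is added in world space.
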(event EventBeginPlay)

(event Collision|EventActorBeginOverlap
  (params (OtherActor :type Actor%20Object%20Reference)))

(event EventTick
  (params (DeltaSeconds :type Float%20%28single-precision%29))
  (bind _self self)
  (bind _returnvalue (Transformation|GetActorTransform _self))
  (bind (_location _rotation) (Math|Transform|BreakTransform _returnvalue))
  (if (Variables|Default|GetIsActive)
    (bind _output_get (Variables|Default|SetTime (+ DeltaSeconds (Variables|Default|GetTime))))
    (if (>= _output_get (Variables|Default|GetSpawnTime))
      (Variables|Default|SetTime 0.0)
      (Game|SpawnActorfromClass (Variables|Default|GetProjectile) (Math|Transform|MakeTransform (+ (Variables|Default|GetSpawnOffset) _location) _rotation) "Undefined" 0 0))))

(fn ConstructionScript)

(fn Activate
  (Variables|Default|SetIsActive true))